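; BP_ShapeCollectible is a spinning collectible actor tied to the character's set of available shapes.
; Tick yaws it at RotationRate, scaled by delta time.
; On interaction, it loops over the character's ShapeAvailable array and add-uniques each element back into that same array, so nothing new is granted as written.
; The construction script hides the Tetrahedron, Cube and Sphere components, with no logic to reveal one.
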(event `/Game/Blueprints/Interfaces/INF_Interactable.OnCharacterInteract`
  (params (Character :type "/Game/Blueprints/BP_MainCharacter Object Reference"))
  (bind _shapeavailable (`/Game/Blueprints/BP_MainCharacter.ShapeAvailable` Character))
  (for _array_element _shapeavailable
    (`KismetArrayLibrary.Array_AddUnique` _shapeavailable _array_element)))

(event `self.ReceiveTick`
  (params (DeltaSeconds :type "Float (single-precision)"))
  (`self.K2_AddActorWorldRotation` self (`KismetMathLibrary.MakeRotator` 0.0 0.0 (* DeltaSeconds (`self.RotationRate`))) false false))

(fn `UserConstructionScript`
  (`SceneComponent.SetVisibility` (`self.Tetrahedron`) false true)
  (`SceneComponent.SetVisibility` (`self.Cube`) false true)
  (`SceneComponent.SetVisibility` (`self.Sphere`) false true))