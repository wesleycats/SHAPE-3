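; Base enemy Blueprint that wanders the NavMesh and either damages an overlapping character or is destroyed by it.
; AIMoveTo heads to a random navigable point, re-rolled if it matches the current location, and on success or failure calls StartTask, which restarts movement.
; On overlap, the enemy dies if the character has any active ability; otherwise it deals damage, throttled by a DoOnce that resets after DamageDelay.
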(event `self.ReceiveBeginPlay`
  (`self.Move`))

(event `Move`
  (`|AIMoveTo` self (`self.RandomLocation`) null
    (:`OnSuccess`
      _)
    (:`OnFail`
      _))
  (`self.StartTask`))

(event `/Game/Blueprints/Interfaces/INF_Interactable.OnCharacterOverlapped`
  (params (Character :type "/Game/Blueprints/BP_MainCharacter Object Reference"))
  (if (`.IsAnyActive` (`/Game/Blueprints/BP_MainCharacter.GetActiveAbilities` Character))
    (`self.Death`)
    (else
      (`/Engine/EditorBlueprintResources/StandardMacros.DoOnce` false :!label _label
        (:`Completed`
          (`/Game/Blueprints/BP_MainCharacter.TakeDamage` Character)
          (`KismetSystemLibrary.Delay` (`self.DamageDelay`))
          (`self.ResetDamage`))))))

(event `ResetDamage`
  (goto _label :!via `Reset`))

(event `Death`
  (`self.K2_DestroyActor`))

(fn `RandomLocation`
  (returns (RandomLocation :type "Vector Structure"))
  (bind _randomlocation (`NavigationSystemV1.K2_GetRandomLocationInNavigableRadius` (`self.K2_GetActorLocation`) (`self.RandomLocationRadius`) null null :!label _label))
  (if (== _randomlocation (`self.K2_GetActorLocation`) :`ErrorTolerance` 0.1)
    (goto _label)
    (else
      (return _randomlocation))))

(fn `StartTask`
  (`self.Move`))

(fn `UserConstructionScript`)