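; BP_Dasher is an AI character that switches between its inherited move behavior and a faster dash at the player.
; Every tick, a sphere overlap within its vision radius picks Dash if BP_MainCharacter is found, otherwise Move.
; StartTask sets walk speed and runs the chosen task.
; Dash moves to the player's position, then waits and calls StartTask again, whether the move succeeds or fails.
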(event `self.ReceiveBeginPlay`
  (`parent.ReceiveBeginPlay`)
  (set `self.InitialWalkSpeed` (`CharacterMovementComponent.MaxWalkSpeed` (`self.CharacterMovement`))))

(event `/Game/Blueprints/Interfaces/INF_Interactable.OnCharacterInteract`
  (params (Character :type "/Game/Blueprints/BP_MainCharacter Object Reference"))
  (`parent.OnCharacterInteract` Character))

(event `Dash`
  (`|AIMoveTo` self (`self.K2_GetActorLocation` (`GameplayStatics.GetPlayerCharacter` 0)) null 2.0
    (:`OnSuccess`
      _)
    (:`OnFail`
      _))
  (`KismetSystemLibrary.Delay` (`self.TaskDelay`))
  (`self.StartTask`))

(event `self.Move`
  (`parent.Move`))

(event `self.ReceiveTick`
  (params (DeltaSeconds :type "Float (single-precision)"))
  (`self.SetState`))

(fn `SetState`
  (bind (_outactors _returnvalue) (`KismetSystemLibrary.SphereOverlapActors` (`self.K2_GetActorLocation`) (`self.VisionRadius`) (`|MakeArray` "ObjectTypeQuery3" :!type "EObjectTypeQuery Enum") "/Game/Blueprints/BP_MainCharacter.BP_MainCharacter_C"))
  (if _returnvalue
    (set `self.NextTask` "NewEnumerator1")
    (else
      (set `self.NextTask` "NewEnumerator0"))))

(fn `StartTask`
  (switch `/Game/Blueprints/Enums/E_AITask` (`self.NextTask`)
    (:`NewEnumerator0`
      (set `CharacterMovementComponent.MaxWalkSpeed` (`self.InitialWalkSpeed`) (`self.CharacterMovement`))
      (`self.Move`))
    (:`NewEnumerator1`
      (set `CharacterMovementComponent.MaxWalkSpeed` (`self.DashSpeed`) (`self.CharacterMovement`))
      (`self.Dash`))))

(fn `UserConstructionScript`
  (`parent.UserConstructionScript`))