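; BP_Enemy is an enemy pawn that wanders endlessly around the navigable level.
; On BeginPlay it starts a Move loop that sends it via AI MoveTo to a random navmesh point within a set radius of its current location.
; Whether the move succeeds or fails, it waits a configurable delay and then picks a new destination.
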(event `self.ReceiveBeginPlay`
  (`self.Move`))

(event `Move`
  (`|AIMoveTo` self (`self.RandomLocation`) null
    (:`OnSuccess`
      _)
    (:`OnFail`
      _))
  (`KismetSystemLibrary.Delay` (`self.TaskDelay`))
  (`self.Move`))

(fn `RandomLocation`
  (returns (RandomLocation :type "Vector Structure"))
  (bind _randomlocation (`NavigationSystemV1.K2_GetRandomLocationInNavigableRadius` (`self.K2_GetActorLocation`) (`self.RandomLocationRadius`) null null))
  (return _randomlocation))

(fn `UserConstructionScript`)