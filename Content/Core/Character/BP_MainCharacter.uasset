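; Player character that shapeshifts between cube, tetrahedron and sphere on the Ability input, triggering each shape's ability.
; Shape changes check an availability map with fallbacks, swap the mesh, then call Stomp, Dash or SGlide; Stomp and SGlide are empty stubs.
; Dash suspends gravity and uses a looping timer for swept forward offsets until its duration ends.
; Active abilities gate movement and a triple jump that resets on landing.
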(event `InputAction|Ability`
  (params (Key :type "Key Structure"))
  ;[1 1 1] Ability Logic
  (:`Pressed`
    (switch `/Game/Core/Character/E_ShapeList` (`self.CurrentShape`)
      (:`NewEnumerator0`
        (`self.BecomeTetrahedron`))
      (:`NewEnumerator1`
        (`self.BecomeSphere`))
      (:`NewEnumerator2`
        (`self.BecomeCube`)))))

(event `self.ReceiveBeginPlay`
  ;[1 1 1] Initialize Shape and Gravity
  (set `self.InitialGravityScale` (`CharacterMovementComponent.GravityScale` (`self.CharacterMovement`)))
  (`self.BecomeCube`))

(event `InputAxis|MoveRight`
  (params (AxisValue :type "Float (single-precision)"))
  (bind (_isdashing _isstomping) (`self.GetActiveAbilities`))
  (bind (_returnvalue_roll _returnvalue_pitch _returnvalue_yaw) (`KismetMathLibrary.BreakRotator` (`self.GetControlRotation`)))
  ;[1 1 1] Movement
  (if (not (or _isdashing _isstomping))
    (`self.AddMovementInput` (`KismetMathLibrary.GetRightVector` (`KismetMathLibrary.MakeRotator` _returnvalue_roll 0.0 _returnvalue_yaw)) AxisValue)))

(event `InputAxis|MoveForward`
  (params (AxisValue :type "Float (single-precision)"))
  (bind (_isdashing _isstomping) (`self.GetActiveAbilities`))
  (bind (_returnvalue_roll _returnvalue_pitch _returnvalue_yaw) (`KismetMathLibrary.BreakRotator` (`self.GetControlRotation`)))
  ;[1 1 1] Movement
  (if (not (or _isdashing _isstomping))
    (`self.AddMovementInput` (`KismetMathLibrary.GetForwardVector` (`KismetMathLibrary.MakeRotator` 0.0 0.0 _returnvalue_yaw)) AxisValue)))

(event `InputAction|Jump`
  (params (Key :type "Key Structure"))
  ;[1 1 1] JumpLogic
  (:`Pressed`
    (if (not (`.IsAnyActive` (`self.GetActiveAbilities`)))
      (`self.TripleJump`)))
  (:`Released`
    (`self.StopJumping`)))

(event `self.K2_OnMovementModeChanged`
  (params (PrevMovementMode :type "EMovementMode Enum" :default "MOVE_None") (NewMovementMode :type "EMovementMode Enum" :default "MOVE_None") (PrevCustomMode :type Byte) (NewCustomMode :type Byte))
  (`self.ResetJumpCount` PrevMovementMode NewMovementMode))

(event `Dash`
  (bind _charactermovement (`self.CharacterMovement`))
  ;[1 1 1] Dash logic
  (set `self.IsDashing` true)
  (set `CharacterMovementComponent.GravityScale` 0.0 _charactermovement)
  (set `MovementComponent.Velocity` (0.0 0.0 0.0) _charactermovement)
  (bind _returnvalue (`KismetSystemLibrary.K2_SetTimer` null "UpdateDash" (`self.AbilityInterval`) true))
  (set `self.DashTimer` _returnvalue)
  (`KismetSystemLibrary.Delay` (`self.DashDuration`))
  (`self.StopDashing`))

(fn `BecomeCube`
  (if (`self.CheckShapeAvailable` "NewEnumerator0")
    (set `self.CurrentShape` "NewEnumerator0")
    (`StaticMeshComponent.SetStaticMesh` (`self.StaticMesh`) "/Engine/BasicShapes/Cube.Cube")
    (`self.Stomp`)
    (else
      (`self.BecomeSphere`))))

(fn `BecomeSphere`
  (if (`self.CheckShapeAvailable` "NewEnumerator2")
    (set `self.CurrentShape` "NewEnumerator2")
    (`StaticMeshComponent.SetStaticMesh` (`self.StaticMesh`) "/Engine/EngineMeshes/Sphere.Sphere")
    (`self.SGlide`)
    (else
      (`self.BecomeTetrahedron`))))

(fn `BecomeTetrahedron`
  (if (`self.CheckShapeAvailable` "NewEnumerator1")
    (set `self.CurrentShape` "NewEnumerator1")
    (`StaticMeshComponent.SetStaticMesh` (`self.StaticMesh`) "/Engine/BasicShapes/Cone.Cone")
    (`self.Dash`)
    (else
      (`self.BecomeSphere`))))

(fn `CheckShapeAvailable`
  (params (NextShape :type "/Game/Core/Character/E_ShapeList Enum" :default "NewEnumerator0"))
  (returns (IsAvailable :type Boolean))
  (return (`BlueprintMapLibrary.Map_Find` (`self.ShapeAvailable`) NextShape)))

(fn `FirstJump`
  (switch `EMovementMode` (`CharacterMovementComponent.MovementMode` (`self.CharacterMovement`))
    (:`MOVE_Walking`
      (`/Engine/EditorBlueprintResources/StandardMacros.IncrementInt` (`self.JumpAmount`)
        (:`  `
          (`self.Jump`))))
    (:`MOVE_Falling`
      (set `self.JumpMaxCount` 4)
      (`/Engine/EditorBlueprintResources/StandardMacros.IncrementInt` (`self.JumpAmount`)
        (:`  `
          (`self.Jump`))))))

(fn `GetActiveAbilities`
  (returns (IsDashing :type Boolean) (IsStomping :type Boolean) (IsSGliding :type Boolean) (IsAnyActive :type Boolean))
  (bind _isdashing (`self.IsDashing`))
  (bind _isstomping (`self.IsStomping`))
  (bind _issgliding (`self.IsSGliding`))
  (return _isdashing _isstomping _issgliding (or _isdashing _isstomping _issgliding)))

(fn `ResetJumpCount`
  (params (PreviousMode :type "EMovementMode Enum" :default "MOVE_None") (CurrentMode :type "EMovementMode Enum" :default "MOVE_None"))
  (if (and (`|EnumEquality` PreviousMode "MOVE_Falling") (`|EnumEquality` CurrentMode "MOVE_Walking"))
    (set `self.JumpAmount` 0)
    (set `self.JumpMaxCount` 3)))

(fn `SecondJump`
  (`/Engine/EditorBlueprintResources/StandardMacros.IncrementInt` (`self.JumpAmount`)
    (:`  `
      (`self.Jump`))))

(fn `SGlide`)

(fn `Stomp`)

(fn `StopDashing`
  (set `self.IsDashing` false)
  (`KismetSystemLibrary.K2_ClearAndInvalidateTimerHandle` (`self.DashTimer`))
  (set `CharacterMovementComponent.GravityScale` (`self.InitialGravityScale`) (`self.CharacterMovement`)))

(fn `ThirdJump`
  (`/Engine/EditorBlueprintResources/StandardMacros.IncrementInt` (`self.JumpAmount`)
    (:`  `
      (`self.Jump`))))

(fn `TripleJump`
  (switch `int` (`self.JumpAmount`)
    (:`0`
      (`self.FirstJump`))
    (:`1`
      (`self.SecondJump`))
    (:`2`
      (`self.ThirdJump`))))

(fn `UpdateDash`
  (bind (_returnvalue_x _returnvalue_y) (`KismetMathLibrary.BreakVector` (* (`KismetMathLibrary.Normal` (`SceneComponent.GetForwardVector` (`self.CapsuleComponent`))) (`self.DashUpdateDistance`))))
  (`self.K2_AddActorWorldOffset` (`KismetMathLibrary.MakeVector` _returnvalue_x _returnvalue_y) true))

(fn `UserConstructionScript`)